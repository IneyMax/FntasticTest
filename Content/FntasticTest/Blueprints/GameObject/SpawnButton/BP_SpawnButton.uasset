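; BP_SpawnButton is an overlap-triggered world button that broadcasts OnButtonPressed, with audio, material and text feedback for active, reload and default states.
; Entering the capsule presses it only when no reload timer is pending; entering during reload cancels the timer without pressing.
; Leaving shows the reload state and starts a short one-shot timer back to default.
; The construction script applies the button's label text.
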(event `self.Capsule.OnComponentBeginOverlap`
  (params (OverlappedComponent :type "PrimitiveComponent Object Reference") (OtherActor :type "Actor Object Reference") (OtherComp :type "PrimitiveComponent Object Reference") (OtherBodyIndex :type Integer) (bFromSweep :type Boolean) (SweepResult :type "HitResult Structure (by ref)"))
  (if (not (`KismetSystemLibrary.K2_IsValidTimerHandle` (`self.ReloadTimer`)))
    (`PrimitiveComponent.SetMaterial` (`self.StaticMesh`) 0 "/Engine/MapTemplates/Materials/BasicAsset01.BasicAsset01")
    (`self.OnButtonPressed`)
    (`TextRenderComponent.K2_SetText` (`self.TextRenderMassege`) (`self.MassageText_Active`))
    (`AudioComponent.Play` (`self.Audio`) 0.0)
    (else
      (`KismetSystemLibrary.K2_ClearAndInvalidateTimerHandle` (`self.ReloadTimer`)))))

(event `self.Capsule.OnComponentEndOverlap`
  (params (OverlappedComponent :type "PrimitiveComponent Object Reference") (OtherActor :type "Actor Object Reference") (OtherComp :type "PrimitiveComponent Object Reference") (OtherBodyIndex :type Integer))
  (`PrimitiveComponent.SetMaterial` (`self.StaticMesh`) 0 "/Game/FntasticTest/Materials/M_ButtonReload.M_ButtonReload")
  (bind _returnvalue (`KismetSystemLibrary.K2_SetTimerDelegate` (`|CreateDelegate` :!event `Reload`) 1.0))
  (set `self.ReloadTimer` _returnvalue)
  (`TextRenderComponent.K2_SetText` (`self.TextRenderMassege`) (`self.MassageText_Reload`)))

(event `Reload`
  (`PrimitiveComponent.SetMaterial` (`self.StaticMesh`) 0 "/Engine/MapTemplates/Materials/BasicAsset03.BasicAsset03")
  (`KismetSystemLibrary.K2_ClearAndInvalidateTimerHandle` (`self.ReloadTimer`))
  (`TextRenderComponent.K2_SetText` (`self.TextRenderMassege`) (`self.MassageText_Default`)))

(fn `UserConstructionScript`
  (`TextRenderComponent.K2_SetText` (`self.TextRenderButtonNumber`) (`self.ButtonText`)))