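; BP_MoveComponent is a movement component, filed under the Turtle game object, that slides its owning actor along a direction at a set speed.
; MoveStart and MoveStop open and close a gate on Tick, which offsets the owner by Direction times Speed and delta time, without sweep.
; Setters supply Direction and Speed, and StopMoveTimer clears and invalidates a timer handle passed to it.
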(event `self.ReceiveTick`
  (params (DeltaSeconds :type "Float (single-precision)"))
  (`/Engine/EditorBlueprintResources/StandardMacros.Gate` true :!label _label
    (:`Exit`
      (`Actor.K2_AddActorWorldOffset` (`self.GetOwner`) (* (`self.Direction`) (* (`self.Speed`) (`GameplayStatics.GetWorldDeltaSeconds`))) false false))))

(event `MoveStart`
  (goto _label :!via `Open`))

(event `MoveStop`
  (goto _label :!via `Close`))

(fn `SetMoveDirection`
  (params (Direction :type "Vector Structure"))
  (set `self.Direction` Direction))

(fn `SetSpeed`
  (params (Speed :type "Float (double-precision)"))
  (set `self.Speed` Speed))

(fn `Stop Move Timer`
  (params (Timer :type "TimerHandle Structure (by ref)"))
  (`KismetSystemLibrary.K2_ClearAndInvalidateTimerHandle` Timer))