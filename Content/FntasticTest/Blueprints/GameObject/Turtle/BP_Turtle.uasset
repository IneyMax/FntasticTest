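; BP_Turtle is a turtle actor that moves through an assigned move strategy object.
; SetMoveStrategy stores the strategy and hands it the turtle's BPMoveComponent, and MoveStart tells that strategy to begin moving.
; Finish destroys the actor, and the Destroyed event clears the strategy reference.
; The construction script applies the TurtleMaterial variable to one material slot of the static mesh.
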(event `MoveStart`
  (`/Game/FntasticTest/Blueprints/Interface/BPI_Move.MovingBegin` (`self.MoveStrategy`)))

(event `self.ReceiveDestroyed`
  (set `self.MoveStrategy` null))

(fn `Finish`
  (returns (bIsFinished :type Boolean))
  (`self.K2_DestroyActor`)
  (return true))

(fn `Set Move Strategy`
  (params (MoveStrategy :type "/Game/FntasticTest/Blueprints/Interface/BPI_Move Interface"))
  (bind _output_get (set `self.MoveStrategy` MoveStrategy))
  (`/Game/FntasticTest/Blueprints/Interface/BPI_Move.SetMoveComponent` _output_get (`self.BP_MoveComponent`)))

(fn `UserConstructionScript`
  (`PrimitiveComponent.SetMaterial` (`self.StaticMesh`) 2 (`self.TurtleMaterial`)))