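; BP_Move_Base is the base movement strategy for the turtle game object, driving a move component supplied to it.
; SetMoveComponent stores that component, pushes direction and speed into it, and binds to its owner's destruction.
; MovingBegin starts the component's movement, while MovingEnd is an empty hook.
; OnOwnerDestroy stops the component's move timer and clears the reference.
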(event `/Game/FntasticTest/Blueprints/Interface/BPI_Move.SetMoveComponent`
  (params (MoveComponent :type "/Game/FntasticTest/Blueprints/GameObject/Turtle/Components/BP_MoveComponent Object Reference"))
  (bind _output_get (set `self.Move Component` MoveComponent))
  (add `Actor.OnDestroyed` (`ActorComponent.GetOwner` _output_get) (`|CreateDelegate` :!event `OnOwnerDestroy`))
  (`/Game/FntasticTest/Blueprints/GameObject/Turtle/Components/BP_MoveComponent.SetMoveDirection` (`self.Move Component`) (`self.MoveDiraction`))
  (`/Game/FntasticTest/Blueprints/GameObject/Turtle/Components/BP_MoveComponent.SetSpeed` (`self.Move Component`) (`self.Speed`)))

(event `/Game/FntasticTest/Blueprints/Interface/BPI_Move.MovingBegin`
  (`/Game/FntasticTest/Blueprints/GameObject/Turtle/Components/BP_MoveComponent.MoveStart` (`self.Move Component`)))

(event `OnOwnerDestroy`
  (params (DestroyedActor :type "Actor Object Reference"))
  (`/Game/FntasticTest/Blueprints/GameObject/Turtle/Components/BP_MoveComponent.Stop Move Timer` (`self.Move Component`) (`self.Timer`))
  (set `self.Move Component` null))

(fn `MovingEnd`
  (returns (NewParam :type "TimerHandle Structure"))
  (return))