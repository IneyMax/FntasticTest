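; BP_Move_Pause is a turtle movement strategy that makes the turtle move in a stop-and-go rhythm.
; MovingBegin calls its parent, then MoveResume, which starts the MoveComponent and sets a short one-shot timer.
; MoveStop halts the component and sets a longer one-shot timer, so chained timers appear to alternate moving and pausing.
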(event `/Game/FntasticTest/Blueprints/Interface/BPI_Move.MovingBegin`
  (`parent.MovingBegin`)
  (`self.MoveResume`))

(event `MoveResume`
  (bind _returnvalue (`KismetSystemLibrary.K2_SetTimerDelegate` (`|CreateDelegate` :!event `MoveStop`) 0.5))
  (set `self.Timer` _returnvalue)
  (`/Game/FntasticTest/Blueprints/GameObject/Turtle/Components/BP_MoveComponent.MoveStart` (`self.Move Component`)))

(event `MoveStop`
  (bind _returnvalue (`KismetSystemLibrary.K2_SetTimerDelegate` (`|CreateDelegate` :!event `MoveResume`) 1.0))
  (set `self.Timer` _returnvalue)
  (`/Game/FntasticTest/Blueprints/GameObject/Turtle/Components/BP_MoveComponent.MoveStop` (`self.Move Component`)))