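; Turtle movement strategy that moves along its set direction and can reverse it for short back-steps.
; MovingBegin runs the parent logic, then starts forward motion through MoveResume.
; MoveResume and MoveBack pass the normal or negated direction to the move component.
; Each also stores a one-shot timer in a shared variable, with the forward interval twice as long as the backward one.
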(event `/Game/FntasticTest/Blueprints/Interface/BPI_Move.MovingBegin`
  (`parent.MovingBegin`)
  (`self.MoveResume`))

(event `MoveResume`
  (bind _returnvalue (`KismetSystemLibrary.K2_SetTimerDelegate` (`|CreateDelegate` :!event `MoveBack`) 1.0))
  (set `self.Timer` _returnvalue)
  (`/Game/FntasticTest/Blueprints/GameObject/Turtle/Components/BP_MoveComponent.SetMoveDirection` (`self.Move Component`) (`self.MoveDiraction`)))

(event `MoveBack`
  (bind _returnvalue (`KismetSystemLibrary.K2_SetTimerDelegate` (`|CreateDelegate` :!event `MoveResume`) 0.5))
  (set `self.Timer` _returnvalue)
  (`/Game/FntasticTest/Blueprints/GameObject/Turtle/Components/BP_MoveComponent.SetMoveDirection` (`self.Move Component`) (* (`self.MoveDiraction`) -1.0)))