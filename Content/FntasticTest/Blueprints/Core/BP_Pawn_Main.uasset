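; BP_Pawn_Main is a pawn that glides in a straight line across the XY plane to a supplied mouse location.
; MovetoMouseLocation stores the target and a flattened, normalized direction, then opens a Gate on Tick through MoveStart.
; While the gate is open, Tick offsets the actor by speed and delta time without sweeping for collision.
; MoveEnd closes the gate once horizontal distance falls below MoveEndDistance.
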(event `self.ReceiveTick`
  (params (DeltaSeconds :type "Float (single-precision)"))
  (`/Engine/EditorBlueprintResources/StandardMacros.Gate` true :!label _label
    (:`Exit`
      (if (>= (`KismetMathLibrary.VSize` (`KismetMathLibrary.MakeVector` (- (.x (`self.TargetLocation`)) (.x (`self.K2_GetActorLocation`))) (- (.y (`self.TargetLocation`)) (.y (`self.K2_GetActorLocation`))) 0.0)) (`self.MoveEndDistance`))
        (`self.K2_AddActorWorldOffset` (* (`self.MoveDiraction`) (* (`self.MoveSpeed`) (`GameplayStatics.GetWorldDeltaSeconds`))))
        (else
          (`self.Move End`))))))

(event `Move Start`
  (goto _label :!via `Open`))

(event `Move End`
  (goto _label :!via `Close`))

(event `/Game/FntasticTest/Blueprints/Interface/BPI_Pawn.MoveToMouseLocation`
  (params (MouseLocation :type "Vector Structure"))
  (set `self.TargetLocation` MouseLocation)
  (set `self.MoveDiraction` (`KismetMathLibrary.Normal` (`KismetMathLibrary.MakeVector` (- (.x MouseLocation) (.x (`self.K2_GetActorLocation`))) (- (.y MouseLocation) (.y (`self.K2_GetActorLocation`))))))
  (`self.Move Start`))

(fn `UserConstructionScript`)