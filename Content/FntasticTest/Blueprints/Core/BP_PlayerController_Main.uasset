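; BP_PlayerController_Main is a player controller for click-to-move play that also creates the main HUD widget on BeginPlay.
; Releasing SetDestination traces under the cursor against WorldStatic and passes the hit location to the pawn through a MoveToMouseLocation interface message.
; A separate MoveToHitLocation function runs SimpleMoveToLocation when the target is at least MinClickDistance from the pawn, but nothing in this Blueprint calls it.
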(event `self.ReceiveBeginPlay`
  (`self.InitWidget`))

(event `InputAction|SetDestination`
  (params (Key :type "Key Structure"))
  (bind (_hitresult _returnvalue) (`self.GetHitResultUnderCursorForObjects` (`|MakeArray` "ObjectTypeQuery1" :!type "EObjectTypeQuery Enum")))
  (:`Released`
    (if _returnvalue
      (message `/Game/FntasticTest/Blueprints/Interface/BPI_Pawn.MoveToMouseLocation` (`self.K2_GetPawn`) (`.Location` (`GameplayStatics.BreakHitResult` _hitresult))))))

(fn `InitWidget`
  (bind _returnvalue (`|CreateWidget` "/Game/FntasticTest/Blueprints/UI/WBP_MainWidget.WBP_MainWidget_C"))
  (bind _output_get (set `self.MainWidget` _returnvalue))
  (`UserWidget.AddToViewport` _output_get 0))

(fn `MoveToHitLocation`
  (params (Location :type "Vector Structure"))
  (if (>= (`KismetMathLibrary.VSize` (- (`self.K2_GetActorLocation` (`self.K2_GetPawn`)) Location)) (`self.MinClickDistance`))
    (`AIBlueprintHelperLibrary.SimpleMoveToLocation` self Location)))

(fn `UserConstructionScript`)